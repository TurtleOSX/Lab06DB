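; BP_Character is a player character with mouse look, strafe movement, gaze-based interaction and click-to-teleport.
; Each tick, GazeCheck line-traces forward from the camera, with debug drawing, and stores any hit actor implementing the Interact interface.
; A click sends InteractMessage to that actor, or otherwise teleports the character to the trace's hit location with zero rotation.
; Forward movement logic exists but is not connected to an event.
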(event `InputAction|MouseClick`
  (params (Key :type "Key Structure"))
  (bind _interactingactor (`self.InteractingActor`))
  (:`Pressed`
    (`/Engine/EditorBlueprintResources/StandardMacros.IsValid` _interactingactor
      (:`Is Valid`
        (message `/Game/Blueprints/Interact.Interact` _interactingactor))
      (:`Is Not Valid`
        (`self.K2_TeleportTo` (`.Location` (`GameplayStatics.BreakHitResult` (stale `GazeCheck` _outhit))))))))

(event `InputAxis|MouseClick`
  (params (AxisValue :type "Float (single-precision)")))

(event `self.ReceiveTick`
  (params (DeltaSeconds :type "Float (single-precision)"))
  (`self.GazeCheck`))

(event `InputAxis|mouseX`
  (params (AxisValue :type "Float (single-precision)"))
  ;[1 1 1] Input
  (`self.AddControllerYawInput` AxisValue))

(event `InputAxis|MoveLeftRight`
  (params (AxisValue :type "Float (single-precision)"))
  ;[1 1 1] Input
  (`self.AddMovementInput` (`self.GetActorRightVector`) AxisValue))

(event `InputAxis|mouseY`
  (params (AxisValue :type "Float (single-precision)"))
  ;[1 1 1] Input
  (`self.AddControllerPitchInput` AxisValue))

(event `GazeCheck`
  (bind _camera (`self.Camera`))
  (bind _returnvalue (`SceneComponent.K2_GetComponentLocation` _camera))
  ;[1 1 1] Gaze check
  (bind _outhit (`KismetSystemLibrary.LineTraceSingle` :`Start` _returnvalue :`End` (+ _returnvalue (* (`SceneComponent.GetForwardVector` _camera) 2000)) :`TraceChannel` "TraceTypeQuery1" :`DrawDebugType` "ForOneFrame"))
  (bind (_bblockinghit _binitialoverlap _time _distance _location _impactpoint _normal _impactnormal _physmat _hitactor) (`GameplayStatics.BreakHitResult` _outhit))
  (if (`KismetSystemLibrary.DoesImplementInterface` _hitactor "/Game/Blueprints/Interact.Interact_C")
    (set `self.InteractingActor` _hitactor)
    (else
      (set `self.InteractingActor` null))))

(fn `UserConstructionScript`)