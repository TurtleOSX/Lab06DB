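; Door Blueprint that moves open and closed when it receives an Interact event.
; A timeline drives a lerp of the Door component's relative location between DoorStart and DoorEnd, without sweep.
; The DoorMovement boolean selects whether Interact plays or reverses the timeline, and a FlipFlop on Finished toggles it after each completed move.
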(event `/Game/Blueprints/Interact.Interact`
  (if (`self.Door Movement`)
    (bind (_direction _driver) (`Timeline|Timeline - Door Up` :!label _label)
      (:`Update`
        (`SceneComponent.K2_SetRelativeLocation` (`self.Door`) (`KismetMathLibrary.VLerp` (`self.DoorStart`) (`self.DoorEnd`) _driver) false false))
      (:`Finished`
        (`/Engine/EditorBlueprintResources/StandardMacros.FlipFlop`
          (:`A`
            (set `self.Door Movement` false))
          (:`B`
            (set `self.Door Movement` true)))))
    (else
      (goto _label :!via `Reverse`))))

(fn `UserConstructionScript`)